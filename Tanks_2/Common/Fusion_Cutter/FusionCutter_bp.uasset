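; Grippable Fusion Cutter tool that repairs friendly or team-0 tanks and sabotages enemy ones, with faction material set by actor tag.
; Pickup records the holder's team; the first pickup also spawns a replacement on authority after a delay.
; Tick, throttled by a one-second Delay, checks trigger or left mouse, then heals or sabotages tanks overlapping HealingZone.
; Tank health shows on a widget, alongside flame, spark and sound feedback.
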(event `self.ReceiveBeginPlay`
  (bind _tags (`self.Tags`))
  (bind _throwablemesh (`self.ThrowableMesh`))
  (set `self.SpawnLocation` (`SceneComponent.K2_GetComponentToWorld` (`self.ThrowableMesh`)))
  (if (`KismetArrayLibrary.Array_Contains` _tags "REP")
    (`PrimitiveComponent.SetMaterial` _throwablemesh 0 "/Game/GlutenFighters/Tanks_2/Common/Fusion_Cutter/rep_1st_weap_inf_fusioncutter_Mat.rep_1st_weap_inf_fusioncutter_Mat")
    (elif (`KismetArrayLibrary.Array_Contains` _tags "IMP")
      (`PrimitiveComponent.SetMaterial` _throwablemesh 0 "/Game/GlutenFighters/Tanks_2/Common/Fusion_Cutter/imp_1st_weap_inf_fusioncutter_Mat.imp_1st_weap_inf_fusioncutter_Mat")
      (elif (`KismetArrayLibrary.Array_Contains` _tags "CIS")
        (`PrimitiveComponent.SetMaterial` _throwablemesh 0 "/Game/GlutenFighters/Tanks_2/Common/Fusion_Cutter/cis_1st_weap_inf_fusioncutter_Mat.cis_1st_weap_inf_fusioncutter_Mat")))))

(event `self.GripComponent.OnHandInteractionBeginEvent`
  (params (Interaction :type "Interaction Structure (by ref)"))
  (bind _returnvalue (`ZomboyInteractionLibrary.GetInteractionCharacter` Interaction))
  (`self.SetOwner` _returnvalue)
  (`self.EnableInput` (`ZomboyInteractionLibrary.GetPlayerController` Interaction))
  (`self.K2_DetachFromActor` "KeepRelative")
  (set `self.Picked Up` true)
  (bind _ascs_character (cast `/Game/Core/Player/CS_Character` _returnvalue))
  (bind _ascs_player_state (cast `/Game/Core/GameMode/CS_PlayerState` (`Pawn.PlayerState` _ascs_character)))
  (set `self.Owner Team Number` (`ZomboyPlayerState.TeamNumber` _ascs_player_state))
  (if (`self.NeverPickedUp`)
    (set `self.NeverPickedUp` false)
    (`KismetSystemLibrary.Delay` (`self.RespawnTime`))
    (`/Engine/EditorBlueprintResources/ActorMacros.Switch Has Authority`
      (:`Authority`
        (`|SpawnActorFromClass` (`GameplayStatics.GetObjectClass` self) (`self.SpawnLocation`) "AlwaysSpawn" "OverrideRootScale" null null)))))

(event `self.GripComponent.OnHandInteractionEndEvent`
  (params (Interaction :type "Interaction Structure (by ref)"))
  (`self.DisableInput` (`ZomboyInteractionLibrary.GetPlayerController` Interaction))
  (`ActorComponent.Deactivate` (`self.FusionCutter_Flame2`))
  (`ActorComponent.Deactivate` (`self.FusionCutter_Sparks`)))

(event `self.GripComponent.OnTriggerReleasedEvent`
  (params (MotionController :type "ZomboyMotionControllerComponent Object Reference"))
  (`ActorComponent.Deactivate` (`self.FusionCutter_Flame2`))
  (`ActorComponent.Deactivate` (`self.FusionCutter_Sparks`))
  (set `self.TriggerPulled` false))

(event `self.GripComponent.OnTriggerPressedEvent`
  (params (MotionController :type "ZomboyMotionControllerComponent Object Reference"))
  (`ActorComponent.Activate` (`self.FusionCutter_Flame2`) false)
  (set `self.TriggerPulled` true))

(event `self.ReceiveTick`
  (params (DeltaSeconds :type "Float (single-precision)"))
  (`KismetSystemLibrary.Delay` 1.0)
  (if (or (`self.TriggerPulled`) (> (`self.GetInputAxisValue`) 0.0))
    (`ActorComponent.Activate` (`self.FusionCutter_Flame2`) false)
    (for _array_element (`PrimitiveComponent.GetOverlappingActors` (`self.Healing Zone`) null)
      (bind _astank_base (cast `/Game/GlutenFighters/Tanks_2/Common/Tank_Base` _array_element)
        (:`then`
          (`ActorComponent.Activate` (`self.FusionCutter_Flame2`) false)
          (`ActorComponent.Activate` (`self.FusionCutter_Sparks`) false)
          (bind _output_get (set `self.Target` _array_element))
          (bind _team_number (`/Game/GlutenFighters/Tanks_2/Common/Tank_Base.Team Number` _astank_base))
          (if (== _team_number (`self.Owner Team Number`))
            (`self.Trigger Heal` _output_get :!label _label)
            (elif (== _team_number 0)
              (goto _label)
              (else
                (`self.Trigger Sabotage` _output_get))))
          (`AudioComponent.Play` (`self.Fusion Cutter Sound`) 0.0))
        (:`CastFailed`
          (`ActorComponent.Deactivate` (`self.FusionCutter_Sparks`)))))
    (else
      (`ActorComponent.Deactivate` (`self.FusionCutter_Flame2`))
      (`ActorComponent.Deactivate` (`self.FusionCutter_Sparks`)))))

(event `self.Healing Zone.OnComponentBeginOverlap`
  (params (OverlappedComponent :type "PrimitiveComponent Object Reference") (OtherActor :type "Actor Object Reference") (OtherComp :type "PrimitiveComponent Object Reference") (OtherBodyIndex :type Integer) (bFromSweep :type Boolean) (SweepResult :type "HitResult Structure (by ref)"))
  (cast `/Game/GlutenFighters/Tanks_2/Common/Tank_Base` OtherActor)
  (bind (_cis_tank _imp_tank _rep_tank _newhealth) (`/Game/GlutenFighters/Tanks_2/Common/Tank_Library.CallTankGETHealth` OtherActor))
  (bind _asfusion_cutter_health_hud (cast `/Game/GlutenFighters/Tanks_2/Common/UI/FusionCutter_Health_HUD` (`WidgetComponent.GetWidget` (`self.Menu_UI_WidgetComponent`))))
  (set `/Game/GlutenFighters/Tanks_2/Common/UI/FusionCutter_Health_HUD.Health` (`KismetMathLibrary.FTrunc` _newhealth) _asfusion_cutter_health_hud))

(event `Trigger Heal`
  (params (Target :type "Actor Object Reference"))
  (bind (_cis_tank _imp_tank _rep_tank _newhealth) (`/Game/GlutenFighters/Tanks_2/Common/Tank_Library.CallTankANDIncreaseHealth` Target))
  (`KismetSystemLibrary.PrintString` (`KismetSystemLibrary.GetDisplayName` Target))
  (`self.Update Display` _newhealth))

(event `Update Display`
  (params (`New Health` :type "Float (double-precision)"))
  (bind _asfusion_cutter_health_hud (cast `/Game/GlutenFighters/Tanks_2/Common/UI/FusionCutter_Health_HUD` (`WidgetComponent.GetWidget` (`self.Menu_UI_WidgetComponent`))))
  (set `/Game/GlutenFighters/Tanks_2/Common/UI/FusionCutter_Health_HUD.Health` (`KismetMathLibrary.FTrunc` `New Health`) _asfusion_cutter_health_hud))

(event `Trigger Sabotage`
  (params (Target :type "Actor Object Reference"))
  (bind _sabotagepercentage (`/Game/GlutenFighters/Tanks_2/Common/Tank_Library.CallTankANDSabotage` Target))
  (`self.Update Display` _sabotagepercentage))

(fn `UserConstructionScript`)